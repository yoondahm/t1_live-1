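; Player controller that lets the player switch control between the BP_T1Character actors in the level with the Tab key.
; BeginPlay caches every BP_T1Character in an array and sets game-only input mode.
; Each Tab press increments a running index, wraps it by the array length, and passes it to PossessCharacter.
; PossessCharacter validates the index, then unpossesses the current pawn and possesses the selected character.
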(event EventBeginPlay
  (bind _outactors (Actor|GetAllActorsOfClass "/Game/Blueprints/Characters/BP_T1Character.BP_T1Character_C"))
  (Variables|Default|SetCharacters _outactors)
  (Input|SetInputModeGameOnly self false))

(event EventTick
  (params (DeltaSeconds :type Float%20%28single-precision%29)))

(event Input|KeyboardEvents|Tab
  (params (Key :type Key%20Structure))
  (:Pressed
    (bind _result (Math|Integer|IncrementInt (Variables|Default|GetCharacterIndex))
      (:%20%20
        (CallFunction|PossessCharacter (Math|Integer|%(Integer) _result (Utilities|Array|Length (Variables|Default|GetCharacters))))))))

(fn ConstructionScript)

(fn PossessCharacter
  (params (PossessIndex :type Integer))
  (if (Utilities|Array|IsValidIndex (Variables|Default|GetCharacters) PossessIndex)
    (Pawn|UnPossess)
    (Pawn|Possess (Utilities|Array|Get(acopy) (Variables|Default|GetCharacters) PossessIndex))))