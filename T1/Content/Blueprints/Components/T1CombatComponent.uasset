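; T1CombatComponent is an actor component that gives its owner hit points and lets it deal and receive damage.
; CombatAttack finds the same component on the hit actor and calls its CombatHit, which subtracts damage and clamps HP between zero and MaxHp.
; All changes go through SetHp, which broadcasts OnHpChanged, prints the value and fires OnHpZero at zero or below.
; BeginPlay initializes HP to MaxHp through that setter.
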(event EventBeginPlay
  (CallFunction|SetHp (Variables|Default|GetMaxHp)))

(event EventTick
  (params (DeltaSeconds :type Float%20%28single-precision%29)))

(fn CombatAttack
  (params (HitDamage :type Float%20%28double-precision%29) (HitActor :type Actor%20Object%20Reference))
  (bind _returnvalue (Actor|GetComponentbyClass HitActor "T1CombatComponent_C"))
  (Utilities|IsValid _returnvalue
    (:Is%20Valid
      (CallFunction|CombatHit _returnvalue HitDamage))))

(fn CombatHit
  (params (HitDamage :type Float%20%28double-precision%29))
  (CallFunction|SetHp (Math|Float|Clamp(Float) (- (Variables|Default|GetHp) HitDamage) 0.0 (Variables|Default|GetMaxHp))))

(fn SetHp
  (params (New%20Hp :type Float%20%28double-precision%29))
  (bind _output_get (Variables|Default|SetHp New%20Hp))
  (Default|CallOnHpChanged _output_get (Variables|Default|GetMaxHp))
  (Development|PrintString (Utilities|String|ToString(Float) (Variables|Default|GetHp)))
  (if (<= (Variables|Default|GetHp) 0.0)
    (Default|CallOnHpZero)))